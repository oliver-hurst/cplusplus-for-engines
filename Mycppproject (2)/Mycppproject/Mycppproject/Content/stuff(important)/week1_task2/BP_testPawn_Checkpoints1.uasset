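; Test player pawn, apparently twin-stick style, with Enhanced Input handlers for move, aim, dash and interact.
; Move calls DoMove, dash sets velocity along LastMoveInput, and interact sends DoInteractMessage to MyOverlappedActorRef, while setoverlapactor stores OverlappedActor.
; Aim inputs record mouse or stick state, but Tick is empty and the aim-rotation logic is disconnected.
; A debug key applies self-damage, and HealthComponent's death event prints "dead".
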(event OnDeathEvent(HealthComponent)
  (Development|PrintString "dead"))

(event Custom|set%20overlap%20actor
  (params (overlapped%20actor :type Actor%20Object%20Reference))
  (Variables|Default|SetOverlappedActor overlapped%20actor))

(event Input|EnhancedActionEvents|EnhancedInputActionIA_Action_Interact
  (params (ActionValue :type Boolean) (ElapsedSeconds :type Float%20%28double-precision%29) (TriggeredSeconds :type Float%20%28double-precision%29) (InputAction :type Input%20Action%20Object%20Reference :default "/TwinStick/Input/Actions/IA_Action_Interact.IA_Action_Interact"))
  ;[0.1013 1 0 0.5] Interact
  (Class|CppInteractionMessages|DoInteract(Message) (Variables|Default|GetMyOverlappedActorRef)))

(event Input|EnhancedActionEvents|EnhancedInputActionIA_Action_Move
  (params (ActionValue :type Vector%202D%20Structure) (ElapsedSeconds :type Float%20%28double-precision%29) (TriggeredSeconds :type Float%20%28double-precision%29) (InputAction :type Input%20Action%20Object%20Reference :default "/TwinStick/Input/Actions/IA_Action_Move.IA_Action_Move"))
  ;[0.15 0.15 0.15 0.5] Move
  (Class|MyPawn|DoMove ActionValue))

(event Input|EnhancedActionEvents|EnhancedInputActionIA_Action_MouseAim
  (params (ActionValue :type Vector%202D%20Structure) (ElapsedSeconds :type Float%20%28double-precision%29) (TriggeredSeconds :type Float%20%28double-precision%29) (InputAction :type Input%20Action%20Object%20Reference :default "/TwinStick/Input/Actions/IA_Action_MouseAim.IA_Action_MouseAim"))
  (bind _playercontroller (Variables|Default|GetPlayerController))
  ;[0.15 0.15 0.15 0.5] Aim - Mouse and Stick
  (Variables|Default|SetUsingMouse true)
  (Utilities|IsValid _playercontroller
    (:Is%20Valid
      (Variables|/Script/Engine.PlayerController|SetbShowMouseCursor _playercontroller false))))

(event Input|EnhancedActionEvents|EnhancedInputActionIA_Action_StickAim
  (params (ActionValue :type Vector%202D%20Structure) (ElapsedSeconds :type Float%20%28double-precision%29) (TriggeredSeconds :type Float%20%28double-precision%29) (InputAction :type Input%20Action%20Object%20Reference :default "/TwinStick/Input/Actions/IA_Action_StickAim.IA_Action_StickAim"))
  (bind (_x _y) (Math|Vector2D|BreakVector2D ActionValue))
  (bind _playercontroller (Variables|Default|GetPlayerController))
  ;[0.15 0.15 0.15 0.5] Aim - Mouse and Stick
  (Variables|Default|SetAimAngle (Math|Trig|RadiansToDegrees (Math|Trig|Atan2(Radians) _y (* _x -1.0))))
  (Variables|Default|SetUsingMouse false)
  (Utilities|IsValid _playercontroller
    (:Is%20Valid
      (Variables|/Script/Engine.PlayerController|SetbShowMouseCursor _playercontroller false))))

(event Input|EnhancedActionEvents|EnhancedInputActionIA_Action_Dash
  (params (ActionValue :type Boolean) (ElapsedSeconds :type Float%20%28double-precision%29) (TriggeredSeconds :type Float%20%28double-precision%29) (InputAction :type Input%20Action%20Object%20Reference :default "/TwinStick/Input/Actions/IA_Action_Dash.IA_Action_Dash"))
  ;[0.15 0.15 0.15 0.5] Dash
  (Variables|Default|SetLaunchDirection (Variables|Default|GetLastMoveInput))
  (Variables|/Script/Engine.MovementComponent|SetVelocity (Pawn|GetMovementComponent) (* (Variables|Default|GetLaunchDirection) (Variables|Dash|GetDashImpulse))))

(event EventControllerChanged
  (params (OldController :type Controller%20Object%20Reference) (NewController :type Controller%20Object%20Reference))
  ;[0.15 0.15 0.15 0.5] Update Player Controller Reference
  (bind _asplayer_controller (Utilities|Casting|CastToPlayerController NewController))
  (Variables|Default|SetPlayerController _asplayer_controller))

(event EventTick
  (params (DeltaSeconds :type Float%20%28single-precision%29))
  ;[0.15 0.15 0.15 0.5] Tick - Update Player Direction
)

(event Input|KeyboardEvents|DebugKey0
  (params (Key :type Key%20Structure :default "None") (ActionValue :type Input%20Action%20Value%20Structure))
  (:Pressed
    (Game|Damage|ApplyDamage self 5e+01 0 0)))

(fn ConstructionScript)